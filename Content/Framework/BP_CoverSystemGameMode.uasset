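; Game mode for a cover system project that exposes spawning of red and blue characters.
; On BeginPlay it shows the mouse cursor and adds the WI_SpawningView widget to the viewport.
; SpawnRed and SpawnBlue events delegate to a referenced SpawningController, which spawns BP_RedCharacter or BP_BlueCharacter at a random place from that team's spawn pool.
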(event Custom|SpawnBlue
  (bind _spawningcontroller (Variables|Default|GetSpawningController))
  (bind _output (Utilities|ResolveSoftReference _spawningcontroller))
  (Class|SpawningController|SpawnActoratRandomPlace _output "/Game/AICharacter/BP_BlueCharacter.BP_BlueCharacter_C" (Variables|/Script/CoverSystem.SpawningController|GetBlueSpawnPlaces _output)))

(event Custom|SpawnRed
  (bind _spawningcontroller (Variables|Default|GetSpawningController))
  (bind _output (Utilities|ResolveSoftReference _spawningcontroller))
  (Class|SpawningController|SpawnActoratRandomPlace _output "/Game/AICharacter/BP_RedCharacter.BP_RedCharacter_C" (Variables|/Script/CoverSystem.SpawningController|GetRedSpawnPlaces _output)))

(event EventBeginPlay
  (Variables|/Script/Engine.PlayerController|SetbShowMouseCursor (Game|GetPlayerController 0) true)
  (bind _returnvalue (UserInterface|CreateWidget "/Game/WI_SpawningView.WI_SpawningView_C"))
  (UserInterface|Viewport|AddtoViewport _returnvalue 0))

(fn ConstructionScript)